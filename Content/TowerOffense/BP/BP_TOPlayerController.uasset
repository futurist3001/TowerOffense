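; Player controller for the Tower Offense game that manages the scope HUD and the end-of-game screen.
; On BeginPlay it binds to the game mode's end-game event and shows a scope widget, which the R key toggles via a FlipFlop.
; When the game ends, it creates the win/lose widget on the next tick and pauses the game.
; A separate event switches input to UI-only with a visible cursor.
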(event `LimitPlayerMovement`
  (bind _returnvalue (`GameplayStatics.GetPlayerController` 0))
  ;[1 1 1] Limit player`s movement
  (`WidgetBlueprintLibrary.SetInputMode_UIOnlyEx` _returnvalue null)
  (set `PlayerController.bShowMouseCursor` true _returnvalue))

(event `self.ReceiveBeginPlay`
  (bind _asbp_togame_mode_base (cast `/Game/TowerOffense/BP/BP_TOGameModeBase` (`GameplayStatics.GetGameMode`)))
  (add `TOGameModeBase.OnEndGame` _asbp_togame_mode_base (delegate `OnEndGame_Event`))
  ;[1 1 1] Create Scope Widget
  (bind _returnvalue (`|CreateWidget` "/Game/TowerOffense/BP/BP_ScopeWidget.BP_ScopeWidget_C" self))
  (set `self.Scope Widget` _returnvalue)
  (`UserWidget.AddToViewport` (`self.Scope Widget`) 0)
  (`Widget.SetVisibility` (`self.Scope Widget`) "Visible" :!label _label))

(event `OnEndGame_Event`
  (params (DelEndGameState :type "EEndGameState Enum" :default "Win"))
  (`KismetSystemLibrary.K2_SetTimerForNextTickDelegate` (delegate `CreateWinLoseWidget`)))

(event `Key|R`
  (params (Key :type "Key Structure"))
  ;[1 1 1] Create Scope Widget
  (:`Pressed`
    (`/Engine/EditorBlueprintResources/StandardMacros.FlipFlop`
      (:`A`
        (goto _label))
      (:`B`
        (`Widget.SetVisibility` (`self.Scope Widget`) "Collapsed")))))

(event `CreateWinLoseWidget`
  (bind _winlosewidget (`self.WinLoseWidget`))
  ;[1 1 1] Create Win/Lose Widget
  (bind _returnvalue (`|CreateWidget` "/Game/TowerOffense/BP/BP_WinLoseWidget.BP_WinLoseWidget_C" self))
  (set `self.WinLoseWidget` _returnvalue)
  (`UserWidget.AddToViewport` _winlosewidget 0)
  (`Widget.SetVisibility` _winlosewidget "Visible")
  (`GameplayStatics.SetGamePaused` true))

(fn `UserConstructionScript`)
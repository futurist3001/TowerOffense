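; Player controller for TowerOffense that creates a scope widget and toggles it on screen.
; On BeginPlay it creates the widget with itself as owner, stores it, adds it to the viewport and makes it visible.
; The R key drives a FlipFlop between visible and collapsed, starting with visible, so the first press leaves the already shown scope unchanged.
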(event `self.ReceiveBeginPlay`
  (bind _returnvalue (`|CreateWidget` "/Game/TowerOffense/BP/BP_ScopeWidget.BP_ScopeWidget_C" self))
  (set `self.ScopeWidget` _returnvalue)
  (`UserWidget.AddToViewport` (`self.ScopeWidget`) 0)
  (`Widget.SetVisibility` (`self.ScopeWidget`) "Visible" :!label _label))

(event `Key|R`
  (params (Key :type "Key Structure"))
  (:`Pressed`
    (`/Engine/EditorBlueprintResources/StandardMacros.FlipFlop`
      (:`A`
        (goto _label))
      (:`B`
        (`Widget.SetVisibility` (`self.ScopeWidget`) "Collapsed")))))

(fn `UserConstructionScript`)